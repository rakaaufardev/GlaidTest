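; Game mode that blacks out the screen at BeginPlay and warms up expensive assets to avoid shader-compilation hitches during gameplay.
; It spawns a time-dilated bomb Niagara system, and on its finish briefly plays sounds and cycles animations on a temporary character.
; A throwaway mesh actor then copies each "preload"-tagged mesh and its materials through a delayed loop macro.
; Afterwards it destroys that actor, waits briefly and calls the PreloadFinished dispatcher.
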(event `self.ReceiveBeginPlay`
  ; Set camera manager / viewport to black screen
  (`PlayerCameraManager.SetManualCameraFade` (`GameplayStatics.GetPlayerCameraManager` 0) 1.0 (struct :`A` 1.0) false)
  (`self.PreloadAssets`))

(event `PreloadAssets`
  ; This event preloads all high-cost (expensive) assets such as Niagara systems, sounds, and large textures at the beginning of the game to ensure smoother performance during gameplay.
  ; This prevents real-time shader compilation, which could cause frame drops.
  ;;[0.15 0.15 0.15 0.5 12] Preload Niagara
  (bind _returnvalue (`NiagaraFunctionLibrary.SpawnSystemAtLocation` "/Game/VFXs/NS_Bomb.NS_Bomb" (`self.PreloadLocation`)))
  (`NiagaraComponent.SetCustomTimeDilation` _returnvalue 4.0)
  (add `NiagaraComponent.OnSystemFinished` _returnvalue (delegate `OnSystemFinished_Event`)))

(event `OnSystemFinished_Event`
  (params (PSystem :type "NiagaraComponent Object Reference"))
  (bind _staticmeshcomponent (`StaticMeshActor.StaticMeshComponent` (`self.PreloadActor`)))
  ; This event preloads all high-cost (expensive) assets such as Niagara systems, sounds, and large textures at the beginning of the game to ensure smoother performance during gameplay.
  ; This prevents real-time shader compilation, which could cause frame drops.
  ;;[0.15 0.15 0.15 0.5 12] Preload Used Audio
  (`self.PreloadAudio` "/Game/SFXs/Metasounds/MS_Breath.MS_Breath")
  (`self.PreloadAudio` "/Game/SFXs/Metasounds/MS_HeartbeatFast.MS_HeartbeatFast")
  (`self.PreloadAudio` "/Game/SFXs/Metasounds/MS_HeartbeatSlow.MS_HeartbeatSlow")
  (`self.PreloadAudio` "/Game/SFXs/Metasounds/MS_Explosion.MS_Explosion")
  (`self.PreloadAudio` "/Game/SFXs/Metasounds/MS_Lock.MS_Lock")
  (`self.PreloadAudio` "/Game/SFXs/Metasounds/MS_Unlock.MS_Unlock")
  (`self.PreloadAudio` "/Game/SFXs/Metasounds/MS_Footstep.MS_Footstep")
  ;;[0.15 0.15 0.15 0.5 12] Preload Used Character Animations
  (bind _returnvalue (`|SpawnActorFromClass` "/Game/Blueprints/Characters/Parent/BP_Character_Base.BP_Character_Base_C" (`KismetMathLibrary.MakeTransform` (`self.PreloadLocation`)) "AdjustIfPossibleButAlwaysSpawn" "MultiplyWithRoot" null null))
  (`KismetSystemLibrary.Delay` 0.2)
  (bind _mesh (`Character.Mesh` _returnvalue))
  (`SkeletalMeshComponent.SetAnimationMode` _mesh "AnimationSingleNode" true)
  (`SkeletalMeshComponent.PlayAnimation` _mesh "/Game/Demo/Characters/Mannequins/Animations/Manny/MM_Idle.MM_Idle" false)
  (`KismetSystemLibrary.Delay` 0.1)
  (`SkeletalMeshComponent.PlayAnimation` _mesh "/Game/Demo/Characters/Mannequins/Animations/Manny/MM_Run_Fwd.MM_Run_Fwd" false)
  (`KismetSystemLibrary.Delay` 0.1)
  (`SkeletalMeshComponent.PlayAnimation` _mesh "/Game/Demo/Characters/Mannequins/Animations/Manny/MM_Walk_Fwd.MM_Walk_Fwd" false)
  (`KismetSystemLibrary.Delay` 0.1)
  (`SkeletalMeshComponent.PlayAnimation` _mesh "/Game/Demo/Characters/Mannequins/Animations/Manny/MM_Walk_InPlace.MM_Walk_InPlace" false)
  (`KismetSystemLibrary.Delay` 0.1)
  (`self.K2_DestroyActor` _returnvalue)
  ;;[0.15 0.15 0.15 0.5 12] Create an actor that will later be used to visualize the expensive mesh on the background
  (bind _returnvalue_2 (`|SpawnActorFromClass` "/Script/Engine.StaticMeshActor" (`KismetMathLibrary.MakeTransform` (`self.PreloadLocation`)) "Undefined" "MultiplyWithRoot" null null))
  (bind _output_get (set `self.PreloadActor` _returnvalue_2))
  (`StaticMeshActor.SetMobility` _output_get "Movable")
  ;;[0.15 0.15 0.15 0.5 12] Loop through all expensive meshes tagged with 'preload', then set the Preload Actor's mesh and materials to match each one.
  ;; Expensive materials include those using Translucent or Masked blend modes, such as glass, fire, or other visual effects (FX
  (bind _outactors (`GameplayStatics.GetAllActorsOfClassWithTag` "/Script/Engine.StaticMeshActor" "preload"))
  (bind _array_element (`self.ForEachLoopCustomWithDelay` _outactors)
    (:`LoopBody`
      (bind _staticmeshcomponent_2 (`StaticMeshActor.StaticMeshComponent` _array_element))
      (`StaticMeshComponent.SetStaticMesh` _staticmeshcomponent (`StaticMeshComponent.StaticMesh` _staticmeshcomponent_2))
      (for (_array_element_2 _array_index) (`MeshComponent.GetMaterials` _staticmeshcomponent_2)
        (`PrimitiveComponent.SetMaterial` _staticmeshcomponent _array_index _array_element_2)))
    (:`Completed`
      ;;[0.15 0.15 0.15 0.5 12] After looping, destroy the preload mesh and call the preload finished dispatcher
      (`self.K2_DestroyActor` (`self.PreloadActor`))
      (`KismetSystemLibrary.Delay` 2.0)
      (`self.PreloadFinished`))))

(fn `UserConstructionScript`)