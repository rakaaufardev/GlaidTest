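; BP_PlayerController creates the player HUD on BeginPlay and opens the player menu through it on the I key.
; It registers with BP_GameMode for the preload-finished callback, holding back game start until assets are ready.
; That callback adds the default Enhanced Input mapping context, fades the camera in from black and plays ambience sound.
; A local-only hotbar widget setup exists but is disconnected and never runs.
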(event `self.ReceiveBeginPlay`
  (`|ExecutionSequence`
    (:`then_0`
      (bind _returnvalue (`|CreateWidget` "/Game/Blueprints/Inventory/WBP_PlayerHUD.WBP_PlayerHUD_C"))
      (bind _output_get (set `self.HUD` _returnvalue))
      (`UserWidget.AddToViewport` _output_get 0)
      ; The game and controller will start after all necessary assets are preloaded in the game mode
      (bind _asbp_game_mode (cast `/Game/Blueprints/Cores/BP_GameMode` (`GameplayStatics.GetGameMode`)))
      (add `/Game/Blueprints/Cores/BP_GameMode.PreloadFinished` _asbp_game_mode (delegate `PreloadFinished_Event`)))))

(event `PreloadFinished_Event`
  ; The game and controller will start after all necessary assets are preloaded in the game mode
  ; Add input to the player controller
  (`EnhancedInputSubsystemInterface.AddMappingContext` (subsystem `EnhancedInputLocalPlayerSubsystem`) "/Game/Demo/Input/IMC_Default.IMC_Default" 0 (struct))
  ; Fade in the game viewport from black
  (`PlayerCameraManager.StartCameraFade` :`self` (`GameplayStatics.GetPlayerCameraManager` 0) :`FromAlpha` 1.0 :`Duration` 1.0 :`bShouldFadeAudio` true)
  ; Play ambience sounds
  (`GameplayStatics.PlaySound2D` (`self.AmbienceSound`) 1.0 1.0 0.0 null null))

(event `Key|I`
  (params (Key :type "Key Structure"))
  (:`Pressed`
    (`/Game/Blueprints/Inventory/WBP_PlayerHUD.DisplayPlayerMenu` (`self.HUD`))))

(fn `UserConstructionScript`)