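; BPIO_Letter is an interactable letter that shows its name and description in the player's item details widget.
; While the player overlaps GlowTrigger, a looping timeline pulses the Glow mesh's emissive parameter forward and back, hiding it briefly between pulses.
; Interact plays a sound and moves input from the pawn to this actor.
; The interact or end-interact input then hides the widget and returns input to the pawn.
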(event `PlayGlow`
  ; Glow For Visual
  (bind (_direction _alpha) (`Timeline|Timeline` :!label _label)
    (:`Update`
      ;;[0.15 0.15 0.15 0.5 12] Uses emissive in the material to make the mesh glow.
      (`MeshComponent.SetScalarParameterValueOnMaterials` (`self.Glow`) "EmissiveBoost" (`KismetMathLibrary.Lerp` 0.0 1000.0 _alpha)))
    (:`Finished`
      ;; After the timeline finished, check if its glowing or not.
      ;; If it's glowing, replay the timeline until its not glowing.
      ;; If it's not glowing, wait for 0.2 seconds, then glow again.
      (switch `ETimelineDirection` _direction
        (:`Forward`
          (`self.ReverseGlow`))
        (:`Backward`
          (`SceneComponent.SetHiddenInGame` (`self.Glow`) true false)
          (`KismetSystemLibrary.Delay` 0.2)
          (`SceneComponent.SetHiddenInGame` (`self.Glow`) false false)
          (`self.PlayGlow`))))))

(event `StopGlow`
  ; Glow For Visual
  (goto _label :!via `Stop`))

(event `ReverseGlow`
  ; Glow For Visual
  (goto _label :!via `Reverse`))

(event `self.GlowTrigger.OnComponentBeginOverlap`
  (params (OverlappedComponent :type "PrimitiveComponent Object Reference") (OtherActor :type "Actor Object Reference") (OtherComp :type "PrimitiveComponent Object Reference") (OtherBodyIndex :type Integer) (bFromSweep :type Boolean) (SweepResult :type "HitResult Structure (by ref)"))
  ; Glow For Visual
  ;; Glowing starts when the player is inside (overlapping) the GlowTrigger.
  ;; If the player exits the trigger, the glowing stops.
  (cast `/Game/Blueprints/Characters/BPC_Player` OtherActor)
  (`SceneComponent.SetHiddenInGame` (`self.Glow`) false false :!label _label_2)
  (`self.PlayGlow`))

(event `self.ReceiveBeginPlay`
  ; Glow For Visual
  ;; Glowing starts when the player is inside (overlapping) the GlowTrigger.
  ;; If the player exits the trigger, the glowing stops.
  (`KismetSystemLibrary.Delay` 0.2)
  (if (`PrimitiveComponent.IsOverlappingActor` (`self.GlowTrigger`) (`GameplayStatics.GetPlayerCharacter` 0))
    (goto _label_2)
    (else
      (`SceneComponent.SetHiddenInGame` (`self.Glow`) true false :!label _label_3)
      (`self.StopGlow`))))

(event `self.GlowTrigger.OnComponentEndOverlap`
  (params (OverlappedComponent :type "PrimitiveComponent Object Reference") (OtherActor :type "Actor Object Reference") (OtherComp :type "PrimitiveComponent Object Reference") (OtherBodyIndex :type Integer))
  ; Glow For Visual
  ;; Glowing starts when the player is inside (overlapping) the GlowTrigger.
  ;; If the player exits the trigger, the glowing stops.
  (cast `/Game/Blueprints/Characters/BPC_Player` OtherActor)
  (goto _label_3))

(event `EnhancedInput|/Game/Demo/Input/Actions/IA_EndInteract`
  (params (ActionValue :type Boolean) (ElapsedSeconds :type "Float (double-precision)") (TriggeredSeconds :type "Float (double-precision)") (InputAction :type "InputAction Object Reference" :default "/Game/Demo/Input/Actions/IA_EndInteract.IA_EndInteract"))
  (bind _returnvalue (`GameplayStatics.GetPlayerController` 0))
  ; If the back key or interact input or end interact input is pressed, hide the item details widget and switch the input receptor back to the player pawn
  (:`Triggered`
    (`/Game/Blueprints/UI/WBP_Gameplay.HideItemDetails` (`/Game/Blueprints/Characters/BPC_Player.GameplayWidget` (`self.Player`)) :!label _label_4)
    (`self.DisableInput` _returnvalue)
    (`self.EnableInput` (`GameplayStatics.GetPlayerPawn` 0) _returnvalue)))

(event `EnhancedInput|/Game/Demo/Input/Actions/IA_Interact`
  (params (ActionValue :type Boolean) (ElapsedSeconds :type "Float (double-precision)") (TriggeredSeconds :type "Float (double-precision)") (InputAction :type "InputAction Object Reference" :default "/Game/Demo/Input/Actions/IA_Interact.IA_Interact"))
  ; If the back key or interact input or end interact input is pressed, hide the item details widget and switch the input receptor back to the player pawn
  (:`Started`
    (goto _label_4)))

(event `/Game/Blueprints/InteractionSystem/Interfaces/BPI_Interactable.Interact`
  (params (Character :type "/Game/Blueprints/Characters/Parent/BP_Character_Base Object Reference"))
  (bind _returnvalue (`GameplayStatics.GetPlayerController` 0))
  ; This event is called by the character interacting with the item.
  ; If the character is the player, play the pickup sound, switch the input receptor to this blueprint, and display the item details widget.
  (set `self.Character` Character)
  (bind _asbpc_player (cast `/Game/Blueprints/Characters/BPC_Player` (`self.Character`)))
  (set `self.Player` _asbpc_player)
  (`GameplayStatics.PlaySound2D` "/Game/SFXs/Metasounds/MS_Lock.MS_Lock" 1.0 1.0 0.0 null null)
  (`self.DisableInput` (`GameplayStatics.GetPlayerPawn` 0) _returnvalue)
  (`self.EnableInput` _returnvalue)
  (`/Game/Blueprints/UI/WBP_Gameplay.ShowItemDetails` (`/Game/Blueprints/Characters/BPC_Player.GameplayWidget` (`self.Player`)) (`self.Name`) (`self.Description`) self))

(fn `UserConstructionScript`
  (`parent.UserConstructionScript`))