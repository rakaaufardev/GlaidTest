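; Parent Blueprint for interactable objects in the interaction system.
; It handles the sprint input itself so character speed stays managed until the input receptor changes.
; IA_Sprint sets a valid Player's MaxWalkSpeed to the CharacterData sprint speed while started or ongoing, and back to walk speed on completion.
; LookAt returns an empty string, and the construction script is empty.
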(event `EnhancedInput|/Game/Demo/Input/Actions/IA_Sprint`
  (params (ActionValue :type Boolean) (ElapsedSeconds :type "Float (double-precision)") (TriggeredSeconds :type "Float (double-precision)") (InputAction :type "InputAction Object Reference" :default "/Game/Demo/Input/Actions/IA_Sprint.IA_Sprint"))
  ; This is necessary to handle the sprint input. By doing this, the controller continues to manage the character's speed until the input receptor changes.
  (:`Started`
    (bind _player (`self.Player` :!label _label)
      (:`then`
        (set `CharacterMovementComponent.MaxWalkSpeed` (`.SprintSpeed_11_CF4C66AF43B82655B8C26F9F4AE1D057` (break `/Game/Blueprints/Characters/Structs/S_CharacterData` (`/Game/Blueprints/Characters/Parent/BP_Character_Base.CharacterData` _player))) (`Character.CharacterMovement` _player)))
      (:`else`)))
  (:`Ongoing`
    (goto _label))
  (:`Completed`
    (bind _player_2 (`self.Player`)
      (:`then`
        (set `CharacterMovementComponent.MaxWalkSpeed` (`.WalkSpeed_12_D72931F44D4711F6C78D14A9FC2B6406` (break `/Game/Blueprints/Characters/Structs/S_CharacterData` (`/Game/Blueprints/Characters/Parent/BP_Character_Base.CharacterData` _player_2))) (`Character.CharacterMovement` _player_2)))
      (:`else`))))

(fn `LookAt`
  (returns (Message :type Text))
  (return ""))

(fn `UserConstructionScript`)