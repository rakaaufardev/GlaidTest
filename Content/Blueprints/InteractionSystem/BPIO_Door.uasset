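; Interactable door that the player can open and close, and that can be locked behind a key.
; On interaction by the player, a locked door checks for its key, then either unlocks and opens or plays a lock sound, showing a HUD notification either way.
; A timeline played forward or in reverse swings the mesh, with collision disabled until the motion finishes.
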(event `Unlock`
  ; Set IsLocked variable to false show unlock notif, play unlock sound and open the door
  (set `self.IsLocked?` false)
  (`/Game/Blueprints/UI/WBP_Gameplay.ShowNotif` (`/Game/Blueprints/Characters/BPC_Player.GameplayWidget` (`self.Player`)) (`|FormatText` "{DoorName} is unlocked" (`self.Name`)))
  (`GameplayStatics.PlaySoundAtLocation` "/Game/SFXs/Metasounds/MS_Unlock.MS_Unlock" (`self.K2_GetActorLocation`) (struct) 1.0 1.0 0.0 null null null null)
  (`self.ToggleOpen/CloseDoor`))

(event `/Game/Blueprints/InteractionSystem/Interfaces/BPI_Interactable.Interact`
  (params (Character :type "/Game/Blueprints/Characters/Parent/BP_Character_Base Object Reference"))
  ; This event is called by the character interacting with the item.
  ; If the character is the player do the event
  (bind _output_get (set `self.Character` Character))
  (bind _asbpc_player (cast `/Game/Blueprints/Characters/BPC_Player` _output_get))
  (set `self.Player` _asbpc_player)
  (if (`self.IsLocked?`)
    ;;[0.15 0.15 0.15 0.5 12] If player have the key, unlock it, if not play lock sound and show locked notification
    (if (`/Game/Blueprints/Characters/Parent/BP_Character_Base.HaveKey` (`self.Player`) (`self.Key`))
      (`self.Unlock`)
      (else
        (`GameplayStatics.PlaySound2D` "/Game/SFXs/Metasounds/MS_Lock.MS_Lock" 1.0 1.0 0.0 null null)
        (`/Game/Blueprints/UI/WBP_Gameplay.ShowNotif` (`/Game/Blueprints/Characters/BPC_Player.GameplayWidget` (`self.Player`)) (`|FormatText` "{DoorName} is locked, you need {key}" (`self.Name`) (`/Game/Blueprints/InteractionSystem/Parents/BP_InteractableObject.Name` (`self.Key`))))))
    (else
      ;;[0.15 0.15 0.15 0.5 12] If its not locked start open the door
      (`self.ToggleOpen/CloseDoor`))))

(event `ToggleOpen/CloseDoor`
  ; Timeline event for open and close the door
  ;;[0.15 0.15 0.15 0.5 12] disable the collision of the door
  (`PrimitiveComponent.SetCollisionEnabled` (`self.StaticMesh`) "NoCollision")
  ;;[0.15 0.15 0.15 0.5 12] Check if the door is in close position or open position
  (if (`self.IsClose`)
    (set `self.IsClose` false)
    ;;[0.15 0.15 0.15 0.5 12] Interpolate the door rotaion with timeline
    (bind (_direction _alpha) (`Timeline|TL_OpenDoor` :!label _label)
      (:`Update`
        (`SceneComponent.K2_SetRelativeRotation` (`self.StaticMesh`) (`KismetMathLibrary.RLerp` (struct) (struct :`Yaw` 120.0) _alpha true) true true))
      (:`Finished`
        ;;;[0.15 0.15 0.15 0.5 12] After the timeline, enable the door collision
        (`PrimitiveComponent.SetCollisionEnabled` (`self.StaticMesh`) "QueryAndPhysics")))
    (else
      (set `self.IsClose` true)
      (goto _label :!via `Reverse`))))

(fn `UserConstructionScript`
  (`parent.UserConstructionScript`))