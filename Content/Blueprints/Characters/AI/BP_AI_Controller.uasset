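; AI controller for bomber enemies that runs BT_AI_Bomber on possessing a BPC_AI_Base pawn and clears its attack target.
; While it has no valid target, perception updates store any detected player in AttackTarget and the blackboard, starting the pawn's bomb timer regardless of distance.
; The same update then copies AttackTarget to every AI sharing its TeamID (unless -1) and starts their bomb timers too.
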(event `self.ReceivePossess`
  (params (PossessedPawn :type "Pawn Object Reference"))
  ; On possess, Set the controlled character, run behavior tree and set attack target to null
  (bind _asbpc_ai_base (cast `/Game/Blueprints/Characters/BPC_AI_Base` PossessedPawn))
  (set `self.ControlledCharacter` _asbpc_ai_base)
  (`self.RunBehaviorTree` "/Game/Blueprints/Characters/AI/BT_AI_Bomber.BT_AI_Bomber")
  (set `self.AttackTarget` null))

(event `self.AIPerception.OnPerceptionUpdated`
  (params (UpdatedActors :type "Array of Actor Object Reference (by ref)"))
  ; Event for perception (only sight perception is active)
  ;;[0.15 0.15 0.15 0.5 12] Check the AttackTarget. if its still null continue the update perception
  (`self.AttackTarget`
    (:`then`)
    (:`else`
      ;;[0.15 0.15 0.15 0.5 12] Check detected actors, if its player then set the attack target
      (for _array_element UpdatedActors
        (bind _asbpc_player (cast `/Game/Blueprints/Characters/BPC_Player` _array_element))
        (bind _output_get (set `self.AttackTarget` _asbpc_player))
        (`BlackboardComponent.SetValueAsObject` (`AIBlueprintHelperLibrary.GetBlackboard` null) "AttackTarget" _output_get)
        ;;;[0.15 0.15 0.15 0.5 12] Begin self-explosion -> triggers no matter how close or far the player is
        (`/Game/Blueprints/Characters/BPC_AI_Base.StartBombTimer` (`self.ControlledCharacter`)))
      ;;[0.15 0.15 0.15 0.5 12] If TeamID = -1, it means it does not have team
      (if (!= (`/Game/Blueprints/Characters/BPC_AI_Base.TeamID` (`self.ControlledCharacter`)) -1)
        ;;[0.15 0.15 0.15 0.5 12] Calling other AI, with the same ID
        (bind _outactors (`GameplayStatics.GetAllActorsOfClass` "/Game/Blueprints/Characters/BPC_AI_Base.BPC_AI_Base_C"))
        (for _array_element_2 _outactors
          (if (== (`/Game/Blueprints/Characters/BPC_AI_Base.TeamID` _array_element_2) (`/Game/Blueprints/Characters/BPC_AI_Base.TeamID` (`self.ControlledCharacter`)))
            (bind _returnvalue (`AIBlueprintHelperLibrary.GetAIController` _array_element_2))
            (bind _asbp_ai_controller (cast `/Game/Blueprints/Characters/AI/BP_AI_Controller` _returnvalue))
            (bind _output_get_2 (set `/Game/Blueprints/Characters/AI/BP_AI_Controller.AttackTarget` (`self.AttackTarget`) _asbp_ai_controller))
            (`BlackboardComponent.SetValueAsObject` (`AIBlueprintHelperLibrary.GetBlackboard` _returnvalue) "AttackTarget" _output_get_2)
            ;;;[0.15 0.15 0.15 0.5 12] Begin self-explosion -> triggers no matter how close or far the player is
            (`/Game/Blueprints/Characters/BPC_AI_Base.StartBombTimer` _array_element_2)))))))

(fn `UserConstructionScript`)