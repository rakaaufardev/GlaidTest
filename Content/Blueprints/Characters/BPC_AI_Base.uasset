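; Base AI character for suicide-bomber enemies that sprint between random patrol points and explode to hurt the player.
; The Behavior Tree calls Attack, which slows the character's time dilation and plays a rate-compensated emissive glow timeline before exploding.
; A separately started bomb timer also detonates it, regardless of player distance.
; Explosion spawns Niagara and sound, applies near or far overlap-based damage and HUD blur, then destroys the actor.
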(event `self.ReceiveBeginPlay`
  ; By default, set the walk speed of the AI to be sprint
  (`parent.ReceiveBeginPlay`)
  (set `CharacterMovementComponent.MaxWalkSpeed` (`.SprintSpeed_11_CF4C66AF43B82655B8C26F9F4AE1D057` (break `/Game/Blueprints/Characters/Structs/S_CharacterData` (`self.CharacterData`))) (`self.CharacterMovement`))
  (`self.GuardPatrol`))

(event `StartBombTimer`
  ; Begin bomb timer (self-explosion) — triggers no matter how close or far the player is
  (bind _returnvalue (`KismetSystemLibrary.K2_SetTimerDelegate` (delegate `BombTimerEvent`) (`self.TimeUntilExplode`)))
  (set `self.BombTimer` _returnvalue))

(event `self.Attack`
  ; Attack Event
  ; This event is called by the Behavior Tree.
  ; In this game, the default attack causes the character to explode.
  ;;[0.15 0.15 0.15 0.5 12] Applies custom time dilation to slow the character to 10% speed before triggering the explosion.
  (set `self.CustomTimeDilation` 0.01)
  ;;[0.15 0.15 0.15 0.5 12] Because the time dilation has changed, the timeline's play rate should be adjusted accordingly.
  (`TimelineComponent.SetPlayRate` (`self.TL_Explode`) (/ 1.0 (`self.CustomTimeDilation`)))
  ;;[0.15 0.15 0.15 0.5 12] Before explode change the emissive color material of the character
  (bind (_direction _alpha) (`Timeline|TL_Explode`)
    (:`Update`
      (`MeshComponent.SetScalarParameterValueOnMaterials` (`self.Mesh`) "EmissiveBoost" (`KismetMathLibrary.Lerp` 1.0 1000.0 _alpha)))
    (:`Finished`
      (`self.Explode`))))

(event `BombTimerEvent`
  ; Begin bomb timer (self-explosion) — triggers no matter how close or far the player is
  (`self.Explode`))

(event `Explode`
  ; Explode event
  ;;[0.15 0.15 0.15 0.5 12] Stop the bomb timer, before explode
  (`KismetSystemLibrary.K2_ClearAndInvalidateTimerHandle` (`self.BombTimer`))
  ;;[0.15 0.15 0.15 0.5 12] Spawn the bomb effect and sound on the character mesh
  (bind _returnvalue (`NiagaraFunctionLibrary.SpawnSystemAtLocation` "/Game/VFXs/NS_Bomb.NS_Bomb" (`SceneComponent.GetSocketLocation` (`self.Mesh`) "pelvis") (struct :`Pitch` 90.0)))
  (`GameplayStatics.SpawnSoundAttached` "/Game/SFXs/Metasounds/MS_Explosion.MS_Explosion" _returnvalue "None" (0.0 0.0 0.0) (struct) "KeepRelativeOffset" false 1.0 1.0 0.0 null null)
  ;;[0.15 0.15 0.15 0.5 12] Apply damage to the player, destroy this actor, and detach its AI controller.
  (`self.GivePlayerDamage`)
  (`self.K2_DestroyActor`)
  (`self.DetachFromControllerPendingDestroy`))

(event `GivePlayerDamage`
  ; After explode, give damage to the player if its overlapping with the Bomb_Layer. the damage will be high if player closest to this character.
  (bind _asbpc_player (cast `/Game/Blueprints/Characters/BPC_Player` (`GameplayStatics.GetPlayerCharacter` 0)))
  (if (`PrimitiveComponent.IsOverlappingActor` (`self.Bomb_Layer_Near`) _asbpc_player)
    (bind _healthcomponent (`/Game/Blueprints/Characters/Parent/BP_Character_Base.HealthComponent` _asbpc_player))
    (`/Game/Blueprints/Characters/Components/BP_CharacterAttribute.DecreaseValue` _healthcomponent 40.0)
    (bind _gameplaywidget (`/Game/Blueprints/Characters/BPC_Player.GameplayWidget` _asbpc_player))
    ;;[0.15 0.15 0.15 0.5 12] Temporarily blur the Gameplay Widget.
    (`/Game/Blueprints/UI/WBP_Gameplay.SetBlurForSeconds` _gameplaywidget 50.0)
    (elif (`PrimitiveComponent.IsOverlappingActor` (`self.Bomb_Layer_Far`) _asbpc_player)
      (`/Game/Blueprints/Characters/Components/BP_CharacterAttribute.DecreaseValue` _healthcomponent 20.0)
      (`/Game/Blueprints/UI/WBP_Gameplay.SetBlurForSeconds` _gameplaywidget 30.0))))

(event `GuardPatrol`
  (bind _patrollocation (`self.PatrolLocation`))
  ; Patrol
  (`|AIMoveTo` self (`|GetArrayItem` _patrollocation (`KismetMathLibrary.RandomInteger` (`KismetArrayLibrary.Array_Length` _patrollocation))) null
    (:`OnSuccess`
      (`KismetSystemLibrary.Delay` (`KismetMathLibrary.RandomFloatInRange` 1.0 3.0))
      (`self.GuardPatrol`))))

(fn `UserConstructionScript`
  (`parent.UserConstructionScript`))