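; Enemy AI character that patrols, chases and attacks the player, and can self-destruct on a timer.
; GuardPatrol loops through patrol locations with random pauses; PawnSensing alerts the player and, when chasing is enabled, moves in for a montage attack.
; A retriggerable delay resumes patrol after sight loss.
; Attack and explosion share GivePlayerDamage, where near and far overlap layers scale health loss and HUD blur.
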(event `self.ReceiveBeginPlay`
  ; By default, set the walk speed of the AI to be sprint
  (`parent.ReceiveBeginPlay`)
  (set `CharacterMovementComponent.MaxWalkSpeed` (`.SprintSpeed_11_CF4C66AF43B82655B8C26F9F4AE1D057` (break `/Game/Blueprints/Characters/Structs/S_CharacterData` (`self.CharacterData`))) (`self.CharacterMovement`))
  (`PrimitiveComponent.SetCollisionResponseToChannel` (`self.Mesh`) "ECC_Camera" "ECR_Ignore")
  (`self.GuardPatrol`))

(event `StartBombTimer`
  ; Begin bomb timer (self-explosion) — triggers no matter how close or far the player is
  (bind _returnvalue (`KismetSystemLibrary.K2_SetTimerDelegate` (delegate `BombTimerEvent`) (`self.TimeUntilExplode`)))
  (set `self.BombTimer` _returnvalue))

(event `BombTimerEvent`
  ; Begin bomb timer (self-explosion) — triggers no matter how close or far the player is
  (`self.Explode`))

(event `Explode`
  ; Explode event
  ;;[0.15 0.15 0.15 0.5 12] Stop the bomb timer, before explode
  (`KismetSystemLibrary.K2_ClearAndInvalidateTimerHandle` (`self.BombTimer`))
  ;;[0.15 0.15 0.15 0.5 12] Spawn the bomb effect and sound on the character mesh
  (bind _returnvalue (`NiagaraFunctionLibrary.SpawnSystemAtLocation` "/Game/VFXs/NS_Bomb.NS_Bomb" (`SceneComponent.GetSocketLocation` (`self.Mesh`) "pelvis") (struct :`Pitch` 90.0)))
  (`GameplayStatics.SpawnSoundAttached` "/Game/SFXs/Metasounds/MS_Explosion.MS_Explosion" _returnvalue "None" (0.0 0.0 0.0) (struct) "KeepRelativeOffset" false 1.0 1.0 0.0 null null)
  ;;[0.15 0.15 0.15 0.5 12] Apply damage to the player, destroy this actor, and detach its AI controller.
  (`self.GivePlayerDamage`)
  (`self.K2_DestroyActor`)
  (`self.DetachFromControllerPendingDestroy`))

(event `GivePlayerDamage`
  ; After explode, give damage to the player if its overlapping with the Bomb_Layer. the damage will be high if player closest to this character.
  (bind _asbpc_player (cast `/Game/Blueprints/Characters/BPC_Player` (`GameplayStatics.GetPlayerCharacter` 0)))
  (if (`PrimitiveComponent.IsOverlappingActor` (`self.Bomb_Layer_Near`) _asbpc_player)
    (bind _healthcomponent (`/Game/Blueprints/Characters/Parent/BP_Character_Base.HealthComponent` _asbpc_player))
    (`/Game/Blueprints/Characters/Components/BP_CharacterAttribute.DecreaseValue` _healthcomponent 40.0)
    (bind _gameplaywidget (`/Game/Blueprints/Characters/BPC_Player.GameplayWidget` _asbpc_player))
    ;;[0.15 0.15 0.15 0.5 12] Temporarily blur the Gameplay Widget.
    (`/Game/Blueprints/UI/WBP_Gameplay.SetBlurForSeconds` _gameplaywidget 50.0)
    (elif (`PrimitiveComponent.IsOverlappingActor` (`self.Bomb_Layer_Far`) _asbpc_player)
      (`/Game/Blueprints/Characters/Components/BP_CharacterAttribute.DecreaseValue` _healthcomponent 20.0)
      (`/Game/Blueprints/UI/WBP_Gameplay.SetBlurForSeconds` _gameplaywidget 30.0))))

(event `GuardPatrol`
  (bind _patrollocation (`self.PatrolLocation`))
  ; Patrol
  (set `CharacterMovementComponent.MaxWalkSpeed` 400.0 (`self.CharacterMovement`))
  (`|AIMoveTo` self (`|GetArrayItem` _patrollocation (`self.Locations`)) null
    (:`OnSuccess`
      (`KismetSystemLibrary.Delay` (`KismetMathLibrary.RandomFloatInRange` 1.0 3.0))
      (`self.GuardPatrol`)
      (`/Engine/EditorBlueprintResources/StandardMacros.IncrementInt` (`self.Locations`)
        (:`  `
          (if (== (`self.Locations`) (`KismetMathLibrary.RandomInteger` (`KismetArrayLibrary.Array_Length` _patrollocation)))
            (set `self.Locations` 0)))))))

(event `self.PawnSensing.OnSeePawn`
  (params (Pawn :type "Pawn Object Reference"))
  ; Comment
  (set `self.Can Attack?` true)
  (`|ExecutionSequence`
    (:`then_0`
      (`|ExecutionSequence`
        (:`then_0`
          (`/Engine/EditorBlueprintResources/StandardMacros.DoOnce` false :!label _label
            (:`Completed`
              (message `/Game/Blueprints/DetectionSystem/BPI_Detection.StartDetection` Pawn self))))
        (:`then_1`
          (if (`self.Should Chase?`)
            (`|AIMoveTo` self (0.0 0.0 0.0) Pawn
              (:`OnSuccess`
                (if (`self.Can Attack?`)
                  (set `self.Can Attack?` false)
                  (`self.Attack`))))))))
    (:`then_1`
      (`KismetSystemLibrary.RetriggerableDelay` 0.2)
      (message `/Game/Blueprints/DetectionSystem/BPI_Detection.StopDetection` Pawn)
      (`self.GuardPatrol`)
      (goto _label :!via `Reset`))))

(event `self.StartChase`
  ; Comment
  (set `self.Should Chase?` true))

(event `self.StopChase`
  ; Comment
  (set `self.Should Chase?` false)
  (`self.GuardPatrol`))

(event `self.Attack`
  (`/Engine/EditorBlueprintResources/StandardMacros.DoOnce` false :!label _label_2
    (:`Completed`
      (`self.PlayAnimMontage` "/Game/Blueprints/Characters/ZombieAttack_UE_Montage.ZombieAttack_UE_Montage" 1.5)
      (`KismetSystemLibrary.Delay` 1.0)
      (`GameplayStatics.PlaySound2D` "/Game/Blueprints/Characters/dagger-thrown-into-body-smartsound-fx-1-00-00.dagger-thrown-into-body-smartsound-fx-1-00-00" 1.0 1.0 0.0 null null)
      (`self.GivePlayerDamage`)
      (set `self.Can Attack?` true)
      (goto _label_2 :!via `Reset`))))

(fn `UserConstructionScript`
  (`parent.UserConstructionScript`))