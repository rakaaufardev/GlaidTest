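; BP_CharacterAttribute is a character component that manages a numeric attribute, such as health, between zero and a maximum.
; Instant and timed increases or decreases clamp the value and fire change dispatchers, and GetLostValue returns the missing amount.
; Looping timers drive changes over time, with each new one clearing both timers first.
; Only the timed decrease fires OnValueEmpty, on the tick after reaching zero.
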(event `IncreaseValue`
  (params (IncreaseAmount :type "Float (double-precision)"))
  ; Instantly increase the value
  (set `self.CurrentValue` (`KismetMathLibrary.FClamp` (+ (`self.CurrentValue`) IncreaseAmount) 0.0 (`self.MaxValue`)))
  (`self.OnValueIncrease`))

(event `DecreaseValue`
  (params (DecreaseAmount :type "Float (double-precision)"))
  ; Instantly decreased the value
  (set `self.CurrentValue` (`KismetMathLibrary.FClamp` (- (`self.CurrentValue`) DecreaseAmount) 0.0 (`self.MaxValue`)))
  (`self.OnValueDecrease`))

(event `IncreaseValueOverTime`
  (params (Delay :type "Float (double-precision)" :default 0.5) (IncreaseAmount :type "Float (double-precision)" :default 1.0))
  ; Start increasing the value over time.
  ; Both the delay and the amount increased are specified by user input.
  (`self.ResetTimer`)
  (bind _returnvalue (`KismetSystemLibrary.K2_SetTimerDelegate` (delegate `IncreaseValueTimerEvent`) Delay true true))
  (set `self.IncreaseTimer` _returnvalue))

(event `IncreaseValueTimerEvent`
  ; Start increasing the value over time.
  ; Both the delay and the amount increased are specified by user input.
  (if (< (`self.CurrentValue`) (`self.MaxValue`))
    (set `self.CurrentValue` (`KismetMathLibrary.FClamp` (+ (`self.CurrentValue`) (stale `IncreaseValueOverTime` IncreaseAmount)) 0.0 (`self.MaxValue`)))
    (`self.OnValueIncrease`)
    (else
      (`KismetSystemLibrary.K2_ClearAndInvalidateTimerHandle` (`self.IncreaseTimer`)))))

(event `ResetTimer`
  ; Stop / Reset the timer events
  (`KismetSystemLibrary.K2_ClearAndInvalidateTimerHandle` (`self.IncreaseTimer`))
  (`KismetSystemLibrary.K2_ClearAndInvalidateTimerHandle` (`self.DecreaseTimer`)))

(event `DecreaseValueOverTime`
  (params (Delay :type "Float (double-precision)" :default 0.1) (DecreaseAmount :type "Float (double-precision)" :default 1.0))
  ; Start decreasing the value over time.
  ; Both the delay and the amount decreased are specified by user input.
  (`self.ResetTimer`)
  (bind _returnvalue (`KismetSystemLibrary.K2_SetTimerDelegate` (delegate `DecreaseValueTimerEvent`) Delay true true))
  (set `self.DecreaseTimer` _returnvalue))

(event `DecreaseValueTimerEvent`
  ; Start decreasing the value over time.
  ; Both the delay and the amount decreased are specified by user input.
  (if (> (`self.CurrentValue`) 0.0)
    (set `self.CurrentValue` (`KismetMathLibrary.FClamp` (- (`self.CurrentValue`) (stale `DecreaseValueOverTime` DecreaseAmount)) 0.0 (`self.MaxValue`)))
    (`self.OnValueDecrease`)
    (else
      (`KismetSystemLibrary.K2_ClearAndInvalidateTimerHandle` (`self.DecreaseTimer`))
      (`self.OnValueEmpty`))))

(fn `GetLostValue`
  (returns (ReturnValue :type "Float (double-precision)"))
  ; Returns the difference between maximum and current health to determine how much health has been lost
  (return (- (`self.MaxValue`) (`self.CurrentValue`))))