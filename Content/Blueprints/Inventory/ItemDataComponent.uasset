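; ItemDataComponent is an actor component that makes its owning actor an item the player can pick up into their inventory.
; On BeginPlay it turns on replication for the owner.
; Interactwith passes the item's data row name and quantity to the player character's InventorySystem, then destroys the owner without checking whether the add succeeded.
; LookAt is a stub that returns an empty string.
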(event `self.ReceiveBeginPlay`
  (`Actor.SetReplicates` (`self.GetOwner`) true))

(event `/Game/Blueprints/InteractionSystem/Interfaces/BPI_Interactable.InteractWith`
  (params (PlayerCharacter :type "/Game/Blueprints/Characters/BPC_Player Object Reference"))
  (bind _inventorysystem (`/Game/Blueprints/Characters/Parent/BP_Character_Base.InventorySystem` PlayerCharacter))
  (bind (_itemid_datatable _itemid_rowname) (break `DataTableRowHandle` (`self.ItemID`)))
  (`/Engine/EditorBlueprintResources/StandardMacros.IsValid` _inventorysystem
    (:`Is Valid`
      (`/Game/Blueprints/Inventory/InventorySystem.AddToInventory` _inventorysystem _itemid_rowname (`self.Quantity`))
      (if true
        (`Actor.K2_DestroyActor` (`self.GetOwner`))))))

(fn `LookAt`
  (returns (Message :type Text))
  (return ""))