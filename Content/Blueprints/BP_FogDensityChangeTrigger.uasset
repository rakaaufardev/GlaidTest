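; BP_FogDensityChangeTrigger is a one-shot trigger volume that fades the level's height fog to a target density when the player enters it.
; On box overlap by BPC_Player, it finds the ExponentialHeightFog actor and stores its current density.
; A timeline then lerps the fog component's density toward TargetFogDensity, and the trigger destroys itself when the timeline finishes.
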(event `self.Box.OnComponentBeginOverlap`
  (params (OverlappedComponent :type "PrimitiveComponent Object Reference") (OtherActor :type "Actor Object Reference") (OtherComp :type "PrimitiveComponent Object Reference") (OtherBodyIndex :type Integer) (bFromSweep :type Boolean) (SweepResult :type "HitResult Structure (by ref)"))
  ; If player overlap with the trigger box, then start changing the fog density using timeline
  (bind _asbpc_player (cast `/Game/Blueprints/Characters/BPC_Player` OtherActor))
  (set `self.Player` _asbpc_player)
  (bind _returnvalue (`GameplayStatics.GetActorOfClass` "/Script/Engine.ExponentialHeightFog"))
  (`/Engine/EditorBlueprintResources/StandardMacros.IsValid` _returnvalue
    (:`Is Valid`
      (set `self.Fog` _returnvalue)
      (set `self.InitialFogDensity` (`ExponentialHeightFogComponent.FogDensity` (`ExponentialHeightFog.Component` (`self.Fog`))))
      (bind (_direction _alpha) (`Timeline|TL_ChangeDensity`)
        (:`Update`
          (`ExponentialHeightFogComponent.SetFogDensity` (`ExponentialHeightFog.Component` (`self.Fog`)) (`KismetMathLibrary.Lerp` (`self.InitialFogDensity`) (`self.TargetFogDensity`) _alpha)))
        (:`Finished`
          (`self.K2_DestroyActor`))))))

(fn `UserConstructionScript`)