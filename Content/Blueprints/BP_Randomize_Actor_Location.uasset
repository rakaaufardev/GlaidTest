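; Actor that moves a referenced actor to a random spot from a list of candidate locations when play begins.
; On BeginPlay it makes the target's root component movable, then places it at its own location plus a randomly picked offset from the Locations array.
; The construction script adds an arrow component at each offset to mark the possible positions.
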(event `self.ReceiveBeginPlay`
  (bind _locations (`self.Locations`))
  ; Randomize Start when the game start
  (bind _actortorandomize (`self.ActorToRandomize`)
    (:`then`
      ;;[0.15 0.15 0.15 0.5 12] Set the mobility of the actor to movable
      (`SceneComponent.SetMobility` (`Actor.RootComponent` _actortorandomize) "Movable")
      ;; Set actor location in world
      (`self.K2_SetActorLocation` (`self.ActorToRandomize`) (+ (`self.K2_GetActorLocation`) (`|GetArrayItem` _locations (`KismetMathLibrary.RandomIntegerInRange` 0 (- (`KismetArrayLibrary.Array_Length` _locations) 1)))) false false))
    (:`else`)))

(fn `UserConstructionScript`
  (for _array_element (`self.Locations`)
    (`AddComponent|NODE_AddArrowComponent-0` :`RelativeTransform` (`KismetMathLibrary.MakeTransform` _array_element (struct :`Pitch` 90.0)))))