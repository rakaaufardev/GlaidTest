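; End-of-game trigger volume that finishes the game when the player overlaps its box and lets any key restart it.
; On overlap it fades the camera and audio to black, plays the gameplay widget's end animation and resets the health and stamina timers to freeze those values.
; After a delay matching the animation, it moves input from the player to itself, so any key press reopens the main map.
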(event `Key|AnyKey`
  (params (Key :type "Key Structure"))
  ; If any key is pressed, restart the game
  (:`Pressed`
    (`GameplayStatics.OpenLevelBySoftObjectPtr` "/Game/MainMaps.MainMaps")))

(event `self.Box.OnComponentBeginOverlap`
  (params (OverlappedComponent :type "PrimitiveComponent Object Reference") (OtherActor :type "Actor Object Reference") (OtherComp :type "PrimitiveComponent Object Reference") (OtherBodyIndex :type Integer) (bFromSweep :type Boolean) (SweepResult :type "HitResult Structure (by ref)"))
  (bind _returnvalue (`GameplayStatics.GetPlayerController` 0))
  (bind _endanimationlength (`self.EndAnimationLength`))
  (bind _asbpc_player (cast `/Game/Blueprints/Characters/BPC_Player` OtherActor))
  (set `self.Player` _asbpc_player)
  ; Fade the camera to black.
  (`PlayerCameraManager.StartCameraFade` :`self` (`GameplayStatics.GetPlayerCameraManager` 0) :`ToAlpha` 1.0 :`Duration` _endanimationlength :`bShouldFadeAudio` true :`bHoldWhenFinished` true)
  ; Show the game widget animation
  (`/Game/Blueprints/UI/WBP_Gameplay.ShowGameEnd` (`/Game/Blueprints/Characters/BPC_Player.GameplayWidget` (`self.Player`)))
  ; Stops any changes to the player's health and stamina values.
  (`/Game/Blueprints/Characters/Components/BP_CharacterAttribute.ResetTimer` (`/Game/Blueprints/Characters/Parent/BP_Character_Base.StaminaComponent` (`self.Player`)))
  (`/Game/Blueprints/Characters/Components/BP_CharacterAttribute.ResetTimer` (`/Game/Blueprints/Characters/Parent/BP_Character_Base.HealthComponent` (`self.Player`)))
  ; Delay 2s before switching input receiver.
  (`KismetSystemLibrary.Delay` _endanimationlength)
  ; Disable the input of the player blueprint, then enable the input for this blueprint.
  (`self.DisableInput` (`self.Player`) _returnvalue)
  (`self.EnableInput` _returnvalue))

(fn `UserConstructionScript`)