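; BP_PC_Lost is a player controller that holds back input setup and the opening fade until the game mode finishes preloading assets.
; On BeginPlay it binds to the PreloadFinished event of BP_GM_Lost.
; When that fires, it adds the default Enhanced Input mapping context and fades the camera and audio in from black.
; An ambience sound node is present but disconnected, so it never plays.
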(event `self.ReceiveBeginPlay`
  ; The game and controller will start after all necessary assets are preloaded in the game mode
  (bind _asbp_gm_lost (cast `/Game/PluginAssets/TheAnotherRealm/Blueprints/Cores/BP_GM_Lost` (`GameplayStatics.GetGameMode`)))
  (add `/Game/PluginAssets/TheAnotherRealm/Blueprints/Cores/BP_GM_Lost.PreloadFinished` _asbp_gm_lost (delegate `PreloadFinished_Event`)))

(event `PreloadFinished_Event`
  ; The game and controller will start after all necessary assets are preloaded in the game mode
  ; Add input to the player controller
  (`EnhancedInputSubsystemInterface.AddMappingContext` (subsystem `EnhancedInputLocalPlayerSubsystem`) "/Game/PluginAssets/TheAnotherRealm/Demo/Input/IMC_Default.IMC_Default" 0 (struct))
  ; Fade in the game viewport from black
  (`PlayerCameraManager.StartCameraFade` :`self` (`GameplayStatics.GetPlayerCameraManager` 0) :`FromAlpha` 1.0 :`Duration` 2.0 :`bShouldFadeAudio` true))

(fn `UserConstructionScript`)