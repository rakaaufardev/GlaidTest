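; Base character Blueprint providing shared movement, stamina, death, key and attack behavior for child characters.
; Sprinting swaps walk speed between CharacterData values while a StaminaComponent drains or regenerates, and is refused when stamina is empty.
; The HealthComponent's empty-value dispatcher, bound on BeginPlay, ragdolls the mesh on death.
; A Keys array with a lookup supports locked doors, and Attack is a placeholder for children to override.
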(event `self.ReceiveBeginPlay`
  ; Set default walk speed
  (set `CharacterMovementComponent.MaxWalkSpeed` (`.WalkSpeed_12_D72931F44D4711F6C78D14A9FC2B6406` (break `/Game/PluginAssets/TheAnotherRealm/Blueprints/Characters/Structs/S_CharacterData` (`self.CharacterData`))) (`self.CharacterMovement`))
  ;[0.15 0.15 0.15 0.5 12] We start regenerating/increasing the value if the stamina is below the maximum.
  (`/Game/PluginAssets/TheAnotherRealm/Blueprints/Characters/Components/BP_CharacterAttribute.IncreaseValueOverTime` (`self.StaminaComponent`) 0.5 1.0)
  ;[0.15 0.15 0.15 0.5 12] In BeginPlay, we bind the OnEmptyValue event dispatcher from the HealthComponent. When the health value reaches 0, the player dies
  ; onEmptyValue of health = Death.
  (add `/Game/PluginAssets/TheAnotherRealm/Blueprints/Characters/Components/BP_CharacterAttribute.OnValueEmpty` (`self.HealthComponent`) (delegate `OnDeathEvent`)))

(event `OnDeathEvent`
  ;[0.15 0.15 0.15 0.5 12] In BeginPlay, we bind the OnEmptyValue event dispatcher from the HealthComponent. When the health value reaches 0, the player dies
  ; onEmptyValue of health = Death.
  ;; Do the ragdoll on death
  (`PrimitiveComponent.SetSimulatePhysics` (`self.Mesh`) true)
  (`PrimitiveComponent.SetCollisionEnabled` (`self.Mesh`) "PhysicsOnly"))

(event `StartSprinting`
  ; StartSprinting Event.
  ; When sprinting starts, set the speed to sprint speed and start degenerating stamina.
  ;;[0.15 0.15 0.15 0.5 12] When starting to sprint, check if stamina is greater than 0. If not, cancel sprinting
  (if (> (`/Game/PluginAssets/TheAnotherRealm/Blueprints/Characters/Components/BP_CharacterAttribute.CurrentValue` (`self.StaminaComponent`)) 0.0)
    (set `CharacterMovementComponent.MaxWalkSpeed` (`.SprintSpeed_11_CF4C66AF43B82655B8C26F9F4AE1D057` (break `/Game/PluginAssets/TheAnotherRealm/Blueprints/Characters/Structs/S_CharacterData` (`self.CharacterData`))) (`self.CharacterMovement`))
    (`/Game/PluginAssets/TheAnotherRealm/Blueprints/Characters/Components/BP_CharacterAttribute.DecreaseValueOverTime` (`self.StaminaComponent`) 0.1 1.0)
    (else
      (`self.StopSprinting`))))

(event `AddKey`
  (params (`input value` :type "/Game/PluginAssets/TheAnotherRealm/Blueprints/InteractionSystem/BPIO_Key Object Reference (by ref)"))
  ; Adds a key to the array. The array is checked when attempting to open locked doors.
  (`KismetArrayLibrary.Array_Add` (`self.Keys`) `input value`))

(event `StopSprinting`
  ; StopSprinting Event
  ; When sprinting stops, set the speed to walk speed and start regenerating stamina.
  (set `CharacterMovementComponent.MaxWalkSpeed` (`.WalkSpeed_12_D72931F44D4711F6C78D14A9FC2B6406` (break `/Game/PluginAssets/TheAnotherRealm/Blueprints/Characters/Structs/S_CharacterData` (`self.CharacterData`))) (`self.CharacterMovement`))
  (`self.IncreaseStamina`))

(event `IncreaseStamina`
  ; This event is the default for increasing stamina
  (`/Game/PluginAssets/TheAnotherRealm/Blueprints/Characters/Components/BP_CharacterAttribute.IncreaseValueOverTime` (`self.StaminaComponent`) 0.2 1.0))

(event `Attack`
  ; Attack Event.
  ; This event will be inherited and implemented by child blueprint
  (`KismetSystemLibrary.PrintString` "This event commonly use for Attacking and will be implemented to child blueprint.  if you're seeing this it means the attack event is not implemented yet"))

(fn `HaveKey`
  (params (InputPin :type "Object Object Reference"))
  (returns (output :type Boolean))
  (locals (IsExist :type Boolean))
  ; Check if the key exists in the keys array.
  (set `local.IsExist` false)
  (for _array_element (`self.Keys`)
    (if (== _array_element InputPin)
      (set `local.IsExist` true)
      (break)))
  (return (`local.IsExist`)))

(fn `UserConstructionScript`)